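; Laser projectile actor for a 3D Pang clone, mimicking the original game's rising shot.
; It starts at zero Z scale and stretches its mesh a fixed step every tick while CanScale is set.
; Overlapping a tagged ceiling or platform destroys it; overlapping a Ball also calls that ball's Split.
; Its Destroy function re-enables shooting on the SideScrollerCharacter, so the next shot waits until this one ends.
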(event EventBeginPlay
  (CallFunction|SetScale 0.0))

(event Collision|EventActorBeginOverlap
  (params (OtherActor :type Actor%20Object%20Reference))
  ;[1 1 1] If the laser collides with a platform or the celing, we just destroy it
  (if (or (Actor|ActorHasTag OtherActor "Ceiling") (Actor|ActorHasTag OtherActor "Platform"))
    (CallFunction|Destroy)
    (else
      ;[1 1 1] If the laser collides with a ball, we call the ball's split function and we destroy the laser
      (if (Actor|ActorHasTag OtherActor "Ball")
        (CallFunction|Destroy)
        (bind _asball (Utilities|Casting|CastToBall OtherActor))
        (Default|Split _asball)))))

(event EventTick
  (params (DeltaSeconds :type Float%20%28single-precision%29))
  ;[1 1 1] If the laser hasn't collided, we keep scaling it
  (if (Variables|Default|GetcanScale)
    (CallFunction|ChangeScale 0.1)))

(fn ConstructionScript)

(fn ChangeScale
  (params (Value :type Float%20%28single-precision%29))
  (bind _mesh (Variables|Default|GetMesh))
  (bind _returnvalue (Transformation|GetWorldScale _mesh))
  (bind (_x _y _z) (Math|Vector|BreakVector _returnvalue))
  ;[1 1 1] We scale the laser mesh, so it simulates the vertical movement from original PANG
  (Transformation|SetWorldScale3D _mesh (Math|Vector|MakeVector _x _y (+ Value _z)))
  (return))

(fn SetScale
  (params (Scale :type Float%20%28single-precision%29))
  (bind _mesh (Variables|Default|GetMesh))
  (bind _returnvalue (Transformation|GetWorldScale _mesh))
  (bind (_x _y) (Math|Vector|BreakVector _returnvalue))
  ;[1 1 1] Set the mesh scale to a specific value
  (Transformation|SetWorldScale3D _mesh (Math|Vector|MakeVector _x _y Scale))
  (return))

(fn Destroy
  ;[1 1 1] Every time we destroy the laser, we tell the character that he can shoot again
  (Variables|Default|SetcanScale false)
  (Actor|DestroyActor)
  (bind _asside_scroller_character (Utilities|Casting|CastToSideScrollerCharacter (Game|GetPlayerCharacter 0)))
  (Variables|/Game/SideScrollerBP/Blueprints/SideScrollerCharacter.SideScrollerCharacter_C|SetcanShoot _asside_scroller_character true)
  (return))