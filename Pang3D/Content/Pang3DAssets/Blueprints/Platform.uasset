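; Moving platform actor for the Pang3D game that slides back and forth along its local Y axis.
; On BeginPlay it picks a random direction and speed and stores its starting world Y position.
; Each tick it offsets itself by a fixed step, not scaled by delta time and without sweep.
; It reverses direction on any actor overlap or when its world Y distance from the start reaches Range.
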(event EventBeginPlay
  ;[1 1 1] Random Direction
  (if (> (Math|Random|RandomFloatinRange 0.0 1.0) 0.5)
    (Variables|Default|Setdir 1)
    (else
      (Variables|Default|Setdir -1)))
  ;[1 1 1] Store initial position
  (Variables|Default|SetinitialPos (.Y (Math|Vector|BreakVector (.Location (Math|Transform|BreakTransform (Transformation|GetActorTransform))))))
  ;[1 1 1] Random speed
  (Variables|Default|Setspeed (Math|Random|RandomFloatinRange 0.5 1.5)))

(event EventTick
  (params (DeltaSeconds :type Float%20%28single-precision%29))
  ;[1 1 1] We move every tick
  (Transformation|AddLocalOffset (Variables|Default|GetPlatform) (Math|Vector|MakeVector 0.0 (* (Variables|Default|Getdir) (Variables|Default|Getspeed)) 0.0) false false)
  ;[1 1 1] If we are outside our bounds, we change direction
  (bind _isover (CallFunction|CheckMaxDistance))
  (if _isover
    (CallFunction|ChangeDir)))

(event Collision|EventActorBeginOverlap
  (params (OtherActor :type Actor%20Object%20Reference))
  ;[1 1 1] If we collide with a wall or another platform, we change direction
  (CallFunction|ChangeDir))

(fn ConstructionScript)

(fn CheckMaxDistance
  ;[1 1 1] Check if the platform is outside of the defined bounds
  (return (>= (Math|Float|Absolute(Float) (- (.Y (Math|Vector|BreakVector (.Location (Math|Transform|BreakTransform (Transformation|GetActorTransform))))) (Variables|Default|GetinitialPos))) (Variables|Default|Getrange))))

(fn ChangeDir
  ;[1 1 1] Invert direction
  (Variables|Default|Setdir (* (Variables|Default|Getdir) -1)))