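; Bouncing ball actor for a 3D take on Pang, with a physics sphere scaled by its Size parameter.
; An impulse starts it moving, and each non-ceiling hit applies another, signed by the hit normal and scaled by mass, to simulate Pang's constant-speed bounce.
; Split destroys the ball, updates the player's score and, above minimum size, spawns two smaller balls intended to travel in different directions.
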(event EventBeginPlay
  (CallFunction|AddBallImpulse 1.0))

(event Collision|EventHit
  (params (MyComp :type Primitive%20Component%20Object%20Reference) (Other :type Actor%20Object%20Reference) (OtherComp :type Primitive%20Component%20Object%20Reference) (bSelfMoved :type Boolean) (HitLocation :type Vector :default "0, 0, 0") (HitNormal :type Vector :default "0, 0, 0") (NormalImpulse :type Vector :default "0, 0, 0") (Hit :type Hit%20Result%20Structure%20%28by%20ref%29))
  (bind (_x _y _z) (Math|Vector|BreakVector HitNormal))
  ;[1 1 1] Every time a ball collides, we add an oposite impulse, this way it has a constant velocity simulating the original PANG
  (if (not (Actor|ActorHasTag Other "Ceiling"))
    ;;[1 1 1] Debug only
    (Development|PrintString (Utilities|String|Append (Utilities|GetDisplayName MyComp) ": " (Utilities|GetDisplayName Other)))
    (if (== _y 0.0)
      _
      (else
        (Variables|Default|SetDirection (/ _y (Math|Float|Absolute(Float) _y)))))
    (CallFunction|AddBallImpulse _z)))

(fn ConstructionScript
  (bind _size (Variables|Default|GetSize))
  (bind _returnvalue (/ _size 1.5))
  ;[1 1 1] On construction, we set the size of the ball (it is a parameter)
  (Transformation|SetWorldScale3D (Variables|Default|GetSphere) (Math|Vector|MakeVector _returnvalue _returnvalue _returnvalue)))

(fn Split
  (bind _returnvalue (Transformation|GetActorTransform))
  (bind _size (Variables|Default|GetSize))
  (bind _returnvalue_2 (- _size 1.0))
  ;[1 1 1] Destroy current ball and increase puntuation
  (Actor|DestroyActor)
  (bind _asside_scroller_character (Utilities|Casting|CastToSideScrollerCharacter (Game|GetPlayerCharacter 0)))
  (Default|SetPunt _asside_scroller_character)
  ;[1 1 1] If the ball doesnt have minimum size, we Spawn two more in different directions
  (if (> _size 1.0)
    (Game|SpawnActorfromClass "Ball_C" _returnvalue "Undefined" 0 1.0 _returnvalue_2 0)
    (Game|SpawnActorfromClass "Ball_C" _returnvalue "Undefined" 0 -1.0 _returnvalue_2 0)))

(fn AddBallImpulse
  (params (VerticalDir :type Float%20%28single-precision%29))
  (bind _sphere (Variables|Default|GetSphere))
  (bind _returnvalue (Physics|GetMass _sphere))
  (Physics|AddImpulse _sphere (Math|Vector|MakeVector 0.0 (* (* (Variables|Default|GetDirection) _returnvalue) 2e+02) (* 8e+02 (* _returnvalue (/ VerticalDir (Math|Float|Absolute(Float) VerticalDir))))) "None" false))